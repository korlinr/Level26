(event EventBeginPlay
  (bind _returnvalue (Class|Actor|GetActorRelativeScale3D))
  (bind (_x _y _z) (Math|Vector|BreakVector _returnvalue))
  ;[1 1 1] Initial Size
  (Variables|Default|SetInitialObjSize (+ _x _y _z)))

(fn ConstructionScript
  (bind _staticmesh1 (Variables|Mesh|GetStaticMesh1))
  (Components|StaticMesh|SetStaticMesh _staticmesh1 (Variables|Default|GetObjectMesh))
  (Development|PrintString (Utilities|String|ToString(Float) (Physics|GetMass _staticmesh1))))

(fn ScaleSelf
  (params (ScalingUp :type Boolean) (GunLVL :type Integer) (ScalingDown :type Boolean))
  (bind _returnvalue (Math|Conversions|ToFloat(Integer) 1))
  (bind _staticmesh1 (Variables|Mesh|GetStaticMesh1))
  (Math|Integer|CompareInt GunLVL 2
    (:==
      (Variables|Default|SetMinScale 0.75))
    (:<
      _))
  (if ScalingUp
    (Variables|Default|SetScaleRate 1.01)
    (Math|Float|CompareFloat (+ (.X (Math|Vector|BreakVector (* (Variables|/Script/Engine.SceneComponent|GetRelativeScale3D _staticmesh1) (Variables|Default|GetScaleRate)))) (.Y (Math|Vector|BreakVector (* (Variables|/Script/Engine.SceneComponent|GetRelativeScale3D _staticmesh1) (Variables|Default|GetScaleRate)))) (.Z (Math|Vector|BreakVector (* (Variables|/Script/Engine.SceneComponent|GetRelativeScale3D _staticmesh1) (Variables|Default|GetScaleRate))))) (* (Variables|Default|GetInitialObjSize) (* _returnvalue 1.5))
      (:<
        (Transformation|SetActorScale3D (* (Variables|/Script/Engine.SceneComponent|GetRelativeScale3D _staticmesh1) (Variables|Default|GetScaleRate)) :!label _label)))
    (elif ScalingDown
      (Variables|Default|SetScaleRate 0.99)
      (Math|Float|CompareFloat (+ (.X (Math|Vector|BreakVector (* (Variables|/Script/Engine.SceneComponent|GetRelativeScale3D _staticmesh1) (Variables|Default|GetScaleRate)))) (.Y (Math|Vector|BreakVector (* (Variables|/Script/Engine.SceneComponent|GetRelativeScale3D _staticmesh1) (Variables|Default|GetScaleRate)))) (.Z (Math|Vector|BreakVector (* (Variables|/Script/Engine.SceneComponent|GetRelativeScale3D _staticmesh1) (Variables|Default|GetScaleRate))))) (/ (Variables|Default|GetInitialObjSize) (/ _returnvalue (Variables|Default|GetMinScale)))
        (:>
          (goto _label))))))

(fn InitialSize
  (return 0.0))