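; EndGame is an overlap trigger that checks whether the player has gathered enough crystals to finish the game.
; When a ScaleCharacter enters, it calls that character's EndGame function and compares the returned crystal count with CrystalsNeeded.
; The player HUD's EndGameHUD then receives true when the count meets or exceeds the requirement, or false when it falls short, which also prints the count.
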(event EventActorBeginOverlap
  (params (OtherActor :type Actor%20Object%20Reference))
  (bind _returnvalue (Game|GetPlayerController 0))
  (bind _returnvalue_2 (HUD|GetHUD _returnvalue))
  (bind _asscale_character (Utilities|Casting|CastToScaleCharacter OtherActor))
  (bind _crystalsend (Default|EndGame _asscale_character true))
  (Variables|Default|SetCrystals%20From%20Player _crystalsend)
  (Math|Integer|CompareInt (Variables|Default|GetCrystals%20From%20Player) (Variables|Default|GetCrystalsNeeded)
    (:>
      (bind _asnew_hud (Utilities|Casting|CastToNewHUD _returnvalue_2 :!label _label))
      (Default|EndGameHUD _asnew_hud true))
    (:==
      (goto _label))
    (:<
      (Development|PrintString (Utilities|String|ToString(Integer) (Variables|Default|GetCrystals%20From%20Player)))
      (bind _asnew_hud_2 (Utilities|Casting|CastToNewHUD _returnvalue_2))
      (Default|EndGameHUD _asnew_hud_2 false))))

(fn ConstructionScript)